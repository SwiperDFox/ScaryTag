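; ItemSpawn is an actor Blueprint that spawns a random pickup, apparently a battery or food, when play begins.
; BeginPlay switches on a random integer to call one of three spawn functions, each adding a child actor component through a single-pass loop.
; The random range yields only the battery and food cases, so the SpawnNothing branch, which also adds a component, is effectively unreachable.
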(event `self.ReceiveBeginPlay`
  (switch `int` (`KismetMathLibrary.RandomInteger` 2)
    (:`Default`
      (`self.SpawnNothing` :!label _label))
    (:`0`
      (`self.SpawnIBattery`))
    (:`1`
      (`self.SpawnFood`))
    (:`2`
      (goto _label))))

(fn `SpawnFood`
  (for _ (range 1)
    (`AddComponent|NODE_AddChildActorComponent-1`)))

(fn `SpawnIBattery`
  (for _ (range 1)
    (`AddComponent|NODE_AddChildActorComponent-0`)))

(fn `SpawnNothing`
  (for _ (range 1)
    (`AddComponent|NODE_AddChildActorComponent-4`)))

(fn `UserConstructionScript`)