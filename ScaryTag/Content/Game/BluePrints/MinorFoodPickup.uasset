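; MinorFoodPickup is a food pickup actor that restores some of the player's hunger when touched.
; On box overlap it casts to ThirdPersonCharacter and acts only while PlayerHunger is below a near-full threshold.
; It then adds a fixed amount, caps the value at the maximum, and destroys itself.
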(event `self.Box.OnComponentBeginOverlap`
  (params (OverlappedComponent :type "PrimitiveComponent Object Reference") (OtherActor :type "Actor Object Reference") (OtherComp :type "PrimitiveComponent Object Reference") (OtherBodyIndex :type Integer) (bFromSweep :type Boolean) (SweepResult :type "HitResult Structure (by ref)"))
  (bind _asthird_person_character (cast `/Game/ThirdPersonBP/Blueprints/ThirdPersonCharacter` OtherActor))
  (if (< (`/Game/ThirdPersonBP/Blueprints/ThirdPersonCharacter.Player_Hunger` _asthird_person_character) 90)
    (bind _output_get (set `/Game/ThirdPersonBP/Blueprints/ThirdPersonCharacter.Player_Hunger` (+ (`/Game/ThirdPersonBP/Blueprints/ThirdPersonCharacter.Player_Hunger` _asthird_person_character) 20) _asthird_person_character))
    (if (> _output_get 100)
      (set `/Game/ThirdPersonBP/Blueprints/ThirdPersonCharacter.Player_Hunger` 100 _asthird_person_character)
      (`self.K2_DestroyActor`)
      (else
        (`self.K2_DestroyActor`)))))

(fn `UserConstructionScript`)