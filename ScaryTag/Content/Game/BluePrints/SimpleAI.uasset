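; Ghost enemy AI that wanders, chases characters it sees, and can be worn down by the player's touch.
; Tick starts delayed moves to random reachable points; PawnSensing triggers a retrying chase that pauses the game with a death message on arrival.
; Each ThirdPersonCharacter overlap reduces Health; at zero the ghost destroys itself, adds a child actor component and reduces that player's battery.
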(event `self.ReceiveActorBeginOverlap`
  (params (OtherActor :type "Actor Object Reference"))
  ;[1 1 1] Ghost Kill
  (bind _asthird_person_character (cast `/Game/ThirdPersonBP/Blueprints/ThirdPersonCharacter` OtherActor))
  (`KismetSystemLibrary.PrintString` "You killed Ghost")
  (set `self.Health` (- (`self.Health`) 1.0))
  (if (<= (`self.Health`) 0.0)
    (`self.K2_DestroyActor`)
    (`AddComponent|NODE_AddChildActorComponent-0`)
    (bind _asthird_person_character_2 (cast `/Game/ThirdPersonBP/Blueprints/ThirdPersonCharacter` OtherActor))
    (set `/Game/ThirdPersonBP/Blueprints/ThirdPersonCharacter.PlayerBattery` (- (`/Game/ThirdPersonBP/Blueprints/ThirdPersonCharacter.PlayerBattery` _asthird_person_character_2) 10) _asthird_person_character_2)))

(event `self.PawnSensing.OnSeePawn`
  (params (Pawn :type "Pawn Object Reference"))
  ;[1 1 1] Dead byGhost
  (bind _ascharacter (cast `Character` Pawn))
  (set `self.IsMoving` true)
  (`|AIMoveTo` self (0.0 0.0 0.0) _ascharacter :!label _label
    (:`OnSuccess`
      (`GameplayStatics.SetGamePaused` true)
      (`KismetSystemLibrary.PrintString` "Dead by ghost"))
    (:`OnFail`
      (`KismetSystemLibrary.Delay` 0.2)
      (goto _label))))

(event `self.ReceiveTick`
  (params (DeltaSeconds :type "Float (single-precision)"))
  (`KismetSystemLibrary.Delay` 2.0)
  (if (not (`self.IsMoving`))
    (set `self.IsMoving` true)
    (`|AIMoveTo` self (`NavigationSystemV1.K2_GetRandomReachablePointInRadius` (`self.K2_GetActorLocation`) 1000.0 null null) null
      (:`OnSuccess`
        _)
      (:`OnFail`
        _))
    (set `self.IsMoving` false)))

(fn `UserConstructionScript`)